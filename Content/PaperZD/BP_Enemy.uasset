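; BP_Enemy is a PaperZD 2D enemy character Blueprint that links movement events to its animation state machine.
; Jumping and walking off a ledge jump NormalStateMachine to the Jump and Airborne nodes, while landing sends a land request to the AnimInstance.
; Received damage only prints test debug details.
; A SpawnSmoke function spawns BP_SmokeFX at the sprite's location and rotation with a supplied flipbook.
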(event `self.OnJumped`
  ;[1 1 1] 跳跃事件
  (`PaperZDAnimInstance.JumpToNode` (`self.AnimInstance`) "Jump" "NormalStateMachine"))

(event `self.ReceiveAnyDamage`
  (params (Damage :type "Float (single-precision)") (DamageType :type "DamageType Object Reference") (InstigatedBy :type "Controller Object Reference") (DamageCauser :type "Actor Object Reference"))
  ;[1 1 1] 接收伤害事件【测试】
  (`KismetSystemLibrary.PrintString` (`KismetStringLibrary.Concat_StrStr` "Damage: " (`KismetStringLibrary.Conv_DoubleToString` Damage) "Damage Type: " (`KismetSystemLibrary.GetDisplayName` DamageType) "Instigated By: " (`KismetSystemLibrary.GetDisplayName` InstigatedBy) "Damage Causer: " (`KismetSystemLibrary.GetDisplayName` DamageCauser)) true true (struct :`R` 1.0 :`G` 0.121519 :`B` 0.196222 :`A` 1.0)))

(event `self.OnWalkingOffLedge`
  (params (PreviousFloorImpactNormal :type "Vector Structure (by ref)") (PreviousFloorContactNormal :type "Vector Structure (by ref)") (PreviousLocation :type "Vector Structure (by ref)") (TimeDelta :type "Float (single-precision)"))
  ;[1 1 1] 被动跌落事件
  (`PaperZDAnimInstance.JumpToNode` (`self.AnimInstance`) "Airborne" "NormalStateMachine"))

(event `self.OnLanded`
  (params (Hit :type "HitResult Structure (by ref)"))
  ;[1 1 1] 落地事件
  (message `/Game/BluePrints/BPI_CustomStateRequest.LandRequest` (`self.AnimInstance`)))

(fn `SpawnSmoke`
  (params (Flipbook :type "PaperFlipbook Object Reference"))
  (bind _returnvalue (`|SpawnActorFromClass` "/Game/Effects/Smoke/BP_SmokeFX.BP_SmokeFX_C" (`KismetMathLibrary.MakeTransform` (.location (`SceneComponent.K2_GetComponentToWorld` (`self.Sprite`))) (.rotation (`SceneComponent.K2_GetComponentToWorld` (`self.Sprite`)))) "Undefined" "MultiplyWithRoot" null null))
  (`/Game/Effects/Smoke/BP_SmokeFX.SetFlipbook` _returnvalue Flipbook))

(fn `UserConstructionScript`)
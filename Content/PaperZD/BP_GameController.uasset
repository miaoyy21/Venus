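; Player controller for a PaperZD character that turns Enhanced Input into movement, jump, light/heavy attack, slide and block.
; Actions are relayed to the character's AnimInstance as messages, whose returned state gates jump and slide and scales movement.
; A timeline drives slide velocity along facing X with movement locked, then jumps the state machine to Airborne or Start.
; Another timeline times blocking, and key 0 simulates taking damage.
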(event `self.ReceiveBeginPlay`
  (bind _returnvalue (pcsubsystem `EnhancedInputLocalPlayerSubsystem` self))
  ;[1 1 1] 开始运行事件
  (bind _asbp_character (cast `/Game/PaperZD/BP_Character` (`GameplayStatics.GetPlayerPawn` 0)))
  (set `self.PlayerCharacter` _asbp_character)
  (`/Engine/EditorBlueprintResources/StandardMacros.IsValid` _returnvalue
    (:`Is Valid`
      (`EnhancedInputSubsystemInterface.AddMappingContext` _returnvalue "/Game/Input/IMC_Input.IMC_Input" 0 (struct)))))

(event `Key|Zero`
  (params (Key :type "Key Structure"))
  ;[1 1 1] 【！！！模拟玩家受到伤害！！！】
  (:`Pressed`
    (message `/Game/BluePrints/BPI_CustomStateRequest.HurtRequest` (`PaperZDCharacter.AnimInstance` (`self.PlayerCharacter`)))))

(event `EnhancedInput|/Game/Input/IA_Move`
  (params (ActionValue :type "Vector2D Structure") (ElapsedSeconds :type "Float (double-precision)") (TriggeredSeconds :type "Float (double-precision)") (InputAction :type "InputAction Object Reference" :default "/Game/Input/IA_Move.IA_Move"))
  ;[1 1 1] 移动输入
  (:`Triggered`
    (if (not (`self.IsLockedMovement`))
      (bind _state (message `/Game/BluePrints/BPI_CustomStateRequest.StateRequest` (`PaperZDCharacter.AnimInstance` (`self.PlayerCharacter`))))
      (`Pawn.AddMovementInput` (`self.PlayerCharacter`) (`KismetMathLibrary.GetForwardVector` (`self.GetControlRotation`)) (* (`KismetMathLibrary.SelectFloat` 0.1 1.0 (`|EnumEquality` _state "NewEnumerator0")) (`KismetMathLibrary.BreakVector2D` ActionValue)) false))))

(event `EnhancedInput|/Game/Input/IA_Jump`
  (params (ActionValue :type "Vector2D Structure") (ElapsedSeconds :type "Float (double-precision)") (TriggeredSeconds :type "Float (double-precision)") (InputAction :type "InputAction Object Reference" :default "/Game/Input/IA_Jump.IA_Jump"))
  ;[1 1 1] 跳跃输入
  (:`Started`
    (bind _state (message `/Game/BluePrints/BPI_CustomStateRequest.StateRequest` (`PaperZDCharacter.AnimInstance` (`self.PlayerCharacter`))))
    (if (not (`|EnumEquality` _state "NewEnumerator0"))
      (`Character.Jump` (`self.PlayerCharacter`)))))

(event `EnhancedInput|/Game/Input/IA_LightAttack`
  (params (ActionValue :type Boolean) (ElapsedSeconds :type "Float (double-precision)") (TriggeredSeconds :type "Float (double-precision)") (InputAction :type "InputAction Object Reference" :default "/Game/Input/IA_LightAttack.IA_LightAttack"))
  ;[1 1 1] 攻击输入
  (:`Started`
    (message `/Game/BluePrints/BPI_CustomStateRequest.AtackRequest` (`PaperZDCharacter.AnimInstance` (`self.PlayerCharacter`)) "NewEnumerator0")))

(event `EnhancedInput|/Game/Input/IA_HeavyAttack`
  (params (ActionValue :type Boolean) (ElapsedSeconds :type "Float (double-precision)") (TriggeredSeconds :type "Float (double-precision)") (InputAction :type "InputAction Object Reference" :default "/Game/Input/IA_HeavyAttack.IA_HeavyAttack"))
  ;[1 1 1] 攻击输入
  (:`Started`
    (message `/Game/BluePrints/BPI_CustomStateRequest.AtackRequest` (`PaperZDCharacter.AnimInstance` (`self.PlayerCharacter`)) "NewEnumerator1")))

(event `EnhancedInput|/Game/Input/IA_Slide`
  (params (ActionValue :type Boolean) (ElapsedSeconds :type "Float (double-precision)") (TriggeredSeconds :type "Float (double-precision)") (InputAction :type "InputAction Object Reference" :default "/Game/Input/IA_Slide.IA_Slide"))
  (bind _charactermovement (`Character.CharacterMovement` (`self.PlayerCharacter`)))
  (bind (_returnvalue_x _returnvalue_y _returnvalue_z) (`KismetMathLibrary.BreakVector` (`CharacterMovementComponent.GetLastUpdateVelocity` _charactermovement)))
  ;[1 1 1] 冲刺输入
  (:`Started`
    (bind _state (message `/Game/BluePrints/BPI_CustomStateRequest.StateRequest` (`PaperZDCharacter.AnimInstance` (`self.PlayerCharacter`))))
    (if (not (or (`|EnumEquality` _state "NewEnumerator6") (`|EnumEquality` _state "NewEnumerator2") (`TimelineComponent.IsPlaying` (`self.SlideTimeline`))))
      (`self.LockedMovementRequest` true)
      (message `/Game/BluePrints/BPI_CustomStateRequest.SlideRequest` (`PaperZDCharacter.GetAnimInstance` (`self.PlayerCharacter`)))
      (bind (_direction _alpha) (`Timeline|SlideTimeline` :!via `PlayFromStart`)
        (:`Update`
          (bind _returnvalue (`self.GetForwardRotation`))
          (set `MovementComponent.Velocity` (`KismetMathLibrary.MakeVector` (* (.x _returnvalue) _alpha (`CharacterMovementComponent.MaxWalkSpeed` _charactermovement) 4.0) _returnvalue_y _returnvalue_z) _charactermovement))
        (:`Finished`
          (`self.SlideFinished`))))))

(event `SlideFinished`
  (bind _playercharacter (`self.PlayerCharacter`))
  (bind _animinstance (`PaperZDCharacter.AnimInstance` (`self.PlayerCharacter`)))
  ;[1 1 1] 冲刺结束事件
  (`self.LockedMovementRequest` false)
  (message `/Game/BluePrints/BPI_CustomStateRequest.ClearState` (`PaperZDCharacter.AnimInstance` _playercharacter))
  (if (`NavMovementComponent.IsFalling` (`Character.CharacterMovement` _playercharacter))
    (`PaperZDAnimInstance.JumpToNode` _animinstance "Airborne" "NormalStateMachine")
    (else
      (`PaperZDAnimInstance.JumpToNode` _animinstance "Start" "NormalStateMachine"))))

(event `EnhancedInput|/Game/Input/IA_Block`
  (params (ActionValue :type Boolean) (ElapsedSeconds :type "Float (double-precision)") (TriggeredSeconds :type "Float (double-precision)") (InputAction :type "InputAction Object Reference" :default "/Game/Input/IA_Block.IA_Block"))
  (bind _animinstance (`PaperZDCharacter.AnimInstance` (`self.PlayerCharacter`)))
  ;[1 1 1] 格挡输入
  (:`Started`
    (if (not (`TimelineComponent.IsPlaying` (`self.BlockTimeline`)))
      (message `/Game/BluePrints/BPI_CustomStateRequest.BlockRequest` _animinstance true)
      (`Timeline|BlockTimeline` :!via `PlayFromStart`
        (:`Finished`
          (message `/Game/BluePrints/BPI_CustomStateRequest.BlockRequest` _animinstance false))))))

(event `/Game/BluePrints/BPI_GameController.LockedMovementRequest`
  (params (IsLocked :type Boolean))
  ;[1 1 1] 设定锁定移动输入状态
  (if IsLocked
    (`MovementComponent.StopMovementImmediately` (`Character.CharacterMovement` (`self.PlayerCharacter`)))
    (`TimelineComponent.Stop` (`self.SlideTimeline`))
    (set `self.IsLockedMovement` true)
    (else
      (set `self.IsLockedMovement` false))))

(fn `GetForwardRotation`
  (returns (ReturnValue :type "Vector Structure"))
  (return (`KismetMathLibrary.GetForwardVector` (`self.K2_GetActorRotation` (`self.PlayerCharacter`)))))

(fn `UserConstructionScript`)
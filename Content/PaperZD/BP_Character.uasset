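; BP_Character is a PaperZD 2D character that links jump, fall and landing events to its animation state machine.
; Jumping or walking off a ledge jumps NormalStateMachine to Airborne, while landing jumps it to Landed, stops movement and sets the movement lock on the cached BP_GameController.
; SpawnSmoke spawns a BP_SmokeFX actor at the sprite's location and rotation with a supplied flipbook.
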(event `self.ReceiveBeginPlay`
  ;[1 1 1] 开始运行事件
  (bind _asbp_game_controller (cast `/Game/PaperZD/BP_GameController` (`self.GetController`)))
  (set `self.PlayerController` _asbp_game_controller))

(event `self.OnJumped`
  ;[1 1 1] 跳跃事件
  (`PaperZDAnimInstance.JumpToNode` (`PaperZDAnimationComponent.AnimInstance` (`self.AnimationComponent`)) "Airborne" "NormalStateMachine" :!label _label))

(event `self.OnWalkingOffLedge`
  (params (PreviousFloorImpactNormal :type "Vector Structure (by ref)") (PreviousFloorContactNormal :type "Vector Structure (by ref)") (PreviousLocation :type "Vector Structure (by ref)") (TimeDelta :type "Float (single-precision)"))
  ;[1 1 1] 跳跃事件
  (goto _label))

(event `self.OnLanded`
  (params (Hit :type "HitResult Structure (by ref)"))
  ;[1 1 1] 落地事件
  (`PaperZDAnimInstance.JumpToNode` (`PaperZDAnimationComponent.AnimInstance` (`self.AnimationComponent`)) "Landed" "NormalStateMachine")
  (`MovementComponent.StopMovementImmediately` (`self.CharacterMovement`))
  (set `/Game/PaperZD/BP_GameController.IsLockedMovement` true (`self.PlayerController`)))

(fn `SpawnSmoke`
  (params (Flipbook :type "PaperFlipbook Object Reference"))
  (bind _returnvalue (`|SpawnActorFromClass` "/Game/Effects/Smoke/BP_SmokeFX.BP_SmokeFX_C" (`KismetMathLibrary.MakeTransform` (.location (`SceneComponent.K2_GetComponentToWorld` (`self.Sprite`))) (.rotation (`SceneComponent.K2_GetComponentToWorld` (`self.Sprite`)))) "Undefined" "MultiplyWithRoot" null null))
  (`/Game/Effects/Smoke/BP_SmokeFX.SetFlipbook` _returnvalue Flipbook))

(fn `UserConstructionScript`)
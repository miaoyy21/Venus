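; BP_Other_Character is a PaperZD 2D character that moves along world X and jumps.
; Jumping or walking off a ledge jumps the animation state machine to Airborne; landing jumps it to Landed, stops movement and locks horizontal input.
; The lock is not cleared within this Blueprint.
; SpawnSmoke spawns a BP_SmokeFX at the sprite's location and rotation with a supplied flipbook.
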(event `InputAxis|Move Left/Right`
  (params (AxisValue :type "Float (single-precision)"))
  (if (not (`self.IsLockedMovement`))
    (`self.AddMovementInput` (1.0 0.0 0.0) AxisValue)))

(event `InputAction|Jump`
  (params (Key :type "Key Structure"))
  (:`Pressed`
    (`self.Jump`)))

(event `self.OnJumped`
  (`PaperZDAnimInstance.JumpToNode` (`PaperZDAnimationComponent.AnimInstance` (`self.AnimationComponent`)) "Airborne" "StateMachine" :!label _label))

(event `self.OnWalkingOffLedge`
  (params (PreviousFloorImpactNormal :type "Vector Structure (by ref)") (PreviousFloorContactNormal :type "Vector Structure (by ref)") (PreviousLocation :type "Vector Structure (by ref)") (TimeDelta :type "Float (single-precision)"))
  (goto _label))

(event `self.OnLanded`
  (params (Hit :type "HitResult Structure (by ref)"))
  (`PaperZDAnimInstance.JumpToNode` (`PaperZDAnimationComponent.AnimInstance` (`self.AnimationComponent`)) "Landed" "StateMachine")
  (`MovementComponent.StopMovementImmediately` (`self.CharacterMovement`))
  (set `self.IsLockedMovement` true))

(fn `SpawnSmoke`
  (params (Flipbook :type "PaperFlipbook Object Reference"))
  (bind _returnvalue (`|SpawnActorFromClass` "/Game/Effects/Smoke/BP_SmokeFX.BP_SmokeFX_C" (`KismetMathLibrary.MakeTransform` (.location (`SceneComponent.K2_GetComponentToWorld` (`self.Sprite`))) (.rotation (`SceneComponent.K2_GetComponentToWorld` (`self.Sprite`)))) "Undefined" "MultiplyWithRoot" null null))
  (`/Game/Effects/Smoke/BP_SmokeFX.SetFlipbook` _returnvalue Flipbook))

(fn `UserConstructionScript`)